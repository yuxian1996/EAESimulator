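; CameraBlueprint is an actor that pans across a map from player axis input, presumably carrying the map camera.
; It enables input from player controller 0 on BeginPlay.
; MoveMapX shifts world X and MoveMapY shifts world Z, each clamped to its Min/Max bounds, with MinY and MaxY limiting Z.
; Movement is axis value times Speed per input event, without delta-time scaling or sweep.
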(event Collision|EventActorBeginOverlap
  (params (OtherActor :type Actor%20Object%20Reference)))

(event EventTick
  (params (DeltaSeconds :type Float%20%28single-precision%29)))

(event EventBeginPlay
  (Input|EnableInput (Game|GetPlayerController 0)))

(event Input|AxisEvents|InputAxisMoveMapY
  (params (AxisValue :type Float%20%28single-precision%29))
  (bind _returnvalue (Transformation|GetActorLocation))
  (bind (_x _y _z) (Math|Vector|BreakVector _returnvalue))
  (Transformation|SetActorLocation (Math|Vector|MakeVector _x _y (Math|Float|Clamp(Float) (+ _z (* AxisValue (Variables|Default|GetSpeed))) (Variables|Default|GetMinY) (Variables|Default|GetMaxY))) false false))

(event Input|AxisEvents|InputAxisMoveMapX
  (params (AxisValue :type Float%20%28single-precision%29))
  (bind _returnvalue (Transformation|GetActorLocation))
  (bind (_x _y _z) (Math|Vector|BreakVector _returnvalue))
  (Transformation|SetActorLocation (Math|Vector|MakeVector (Math|Float|Clamp(Float) (+ _x (* AxisValue (Variables|Default|GetSpeed))) (Variables|Default|GetMinX) (Variables|Default|GetMaxX)) _y _z) false false))

(fn ConstructionScript)