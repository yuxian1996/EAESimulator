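; Game instance for the EAE simulator that acts as a central access point for UI panels and gameplay managers.
; On Init it caches the GameLoop actor, and getters forward to its Human, Data, Time and Task managers.
; ShowWidget creates the named panel or menu, stores it in WidgetList and uses the name's integer value as Z-order.
; HideWidget removes the stored widget from its parent; OrderWidget is an empty stub.
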(event EventInit
  (bind _outactors (Actor|GetAllActorsOfClass "/Script/EAESimulator.GameLoop"))
  (for _array_element _outactors
    (Variables|Default|SetGameLoop _array_element)))

(fn ShowWidget
  (params (WidgetName :type WidgetEnum%20Enum :default "NewEnumerator0"))
  (bind _widgetlist (Variables|Default|GetWidgetList))
  (Utilities|IsValid (Game|GetPlayerController 0)
    (:Is%20Valid
      (switch Utilities|FlowControl|Switch|SwitchonWidgetEnum WidgetName
        (:NewEnumerator0
          (bind _returnvalue (UserInterface|CreateWidget "/Game/Blueprints/UMG/PersonPanel/PersonInfo.PersonInfo_C"))
          (Utilities|Map|Add _widgetlist WidgetName _returnvalue)
          (LocalVariables|Setwidget _returnvalue))
        (:NewEnumerator1
          (bind _returnvalue_2 (UserInterface|CreateWidget "/Game/Blueprints/UMG/TaskPanel/TaskBase.TaskBase_C"))
          (Utilities|Map|Add _widgetlist WidgetName _returnvalue_2)
          (LocalVariables|Setwidget _returnvalue_2))
        (:NewEnumerator2
          (bind _returnvalue_3 (UserInterface|CreateWidget "/Game/Blueprints/UMG/MainMenu/MainMenu.MainMenu_C"))
          (Utilities|Map|Add _widgetlist WidgetName _returnvalue_3)
          (LocalVariables|Setwidget _returnvalue_3)))
      (UserInterface|Viewport|AddtoViewport _returnvalue (Math|Conversions|ToInteger(Byte) WidgetName))
      (return (LocalVariables|Getwidget)))))

(fn HideWidget
  (params (Name :type WidgetEnum%20Enum :default "NewEnumerator0"))
  (bind _widgetlist (Variables|Default|GetWidgetList))
  (bind (_value _returnvalue) (Utilities|Map|Find _widgetlist Name))
  (if _returnvalue
    (Widget|RemovefromParent _value)))

(fn OrderWidget)

(fn GetHumanMgr
  (return (Class|GameLoop|GetHumanMgr (Variables|Default|GetGameLoop))))

(fn GetDataMgr
  (return (Class|GameLoop|GetDataMgr (Variables|Default|GetGameLoop))))

(fn GetTimeMgr
  (return (Class|GameLoop|GetTimeMgr (Variables|Default|GetGameLoop))))

(fn GetTaskMgr
  (return (Class|GameLoop|GetTaskMgr (Variables|Default|GetGameLoop))))